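; BP_MIDIManager turns input from a connected MIDI controller into a polyphonic MetaSound synth.
; On BeginPlay it scans MIDI devices, opens the one matching MIDiControllerIndex and binds its events.
; Note On plays a new MSS_Polysynth sound stored in PolyVoices by note number; Note Off triggers that voice's release.
; Control Change handling is unfinished: CC 7 loops voices without effect, while monosynth and parameter-mapping logic sit disconnected.
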(event Custom|EventOnMIDIEvent
  (params (MIDIDeviceController :type MIDI%20Device%20Controller%20Object%20Reference) (Timestamp :type Integer) (EventType :type EMIDIEventType%20Enum :default "Unknown") (Channel :type Integer) (ControlID :type Integer) (Velocity :type Integer) (RawEventType :type Integer))
  (bind _returnvalue (Math|Conversions|ToFloat(Integer) ControlID))
  (bind _returnvalue_2 (Math|Float|Truncate _returnvalue))
  ;[0.0286 0.01701 0.15 0.6783] Event - Vérification de la note te vélocité de la touche pressée + si oui - joue
  ;;[0.15 0.15 0.15 0.5] Imprimer à l'écran
  (Development|PrintString (Utilities|String|ToString(Text) (Utilities|Text|FormatText "MIDI EVENT TYPE {event} MIDI Note {note} Vélocité {vélocité}" ControlID Velocity (Utilities|String|EnumtoString EventType))) true true "(R=0.000000,G=1.000000,B=0.102804,A=1.000000)" 2.0 "MIDI")
  (switch Utilities|FlowControl|Switch|SwitchonEMIDIEventType EventType
    (:NoteOff
      ;[0.15 0.15 0.15 0.5] Arret note
      (Class|AudioParameterControllerInterface|SetTriggerParameter (Utilities|Array|Get(acopy) (Variables|Default|GetPolyVoices) _returnvalue_2) "Trigger Release"))
    (:NoteOn
      (bind _returnvalue_3 (Audio|CreateSound2D "/Game/MetaSound/MSS_Polysynth.MSS_Polysynth" 1.0 1.0 0.0 0))
      (Utilities|Array|SetArrayElem (Variables|Default|GetPolyVoices) _returnvalue_2 _returnvalue_3 true)
      (Audio|Parameter|SetFloatParameter _returnvalue_3 "MIDI Note" _returnvalue :!class /Script/AudioExtensions.AudioParameterControllerInterface)
      (Audio|Components|Audio|Play _returnvalue_3 0.0))
    (:ControlChange
      ;[0.15 0.15 0.15 0.5] autre control change
      (switch string (Utilities|String|ToString(Integer) _returnvalue_2)
        (:7
          (for _array_element (Variables|Default|GetPolyVoices)
            _))))))

(event EventBeginPlay
  ;[0.7396 0.5783 0.09347] Tableau des controleurs MIDI connectés  savoir quel controleur joué - Index -for each + if (branch)
  (bind _outmididevices (Class|MIDIDeviceManager|FindMIDIDevices))
  (for _array_element _outmididevices
    (if (.bCanReceiveFrom (Utilities|Struct|BreakFoundMIDIDevice _array_element))
      (if (== (Variables|Default|GetMIDiControllerIndex) (.DeviceID (Utilities|Struct|BreakFoundMIDIDevice _array_element)))
        (Development|PrintString (.DeviceName (Utilities|Struct|BreakFoundMIDIDevice _array_element)) true true "(R=0.000000,G=0.660000,B=1.000000,A=1.000000)" 3e+01)
        ;[0.7422 0.1991 0.1991 0.5] Création controller MIDI + Création Event
        (bind _returnvalue (Class|MIDIDeviceManager|CreateMIDIDeviceController (.DeviceID (Utilities|Struct|BreakFoundMIDIDevice _array_element)) 1024))
        (bind _output_get (Variables|Default|SetMIDIControl _returnvalue)) ; le MIDI reste tout le temps
        (EventDispatchers|BindEventtoOnMIDIEvent _output_get (EventDispatchers|CreateEvent :!event Custom|EventOnMIDIEvent)))))
  (Development|PrintString "Print terminé" true true "(R=0.000000,G=0.660000,B=1.000000,A=1.000000)" 3e+01))

(fn ConstructionScript)